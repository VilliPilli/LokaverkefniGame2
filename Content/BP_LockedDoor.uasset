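; BP_LockedDoor is a door actor that the first-person character can open only while holding a key.
; Overlapping its box trigger with BP_FirstPersonCharacter caches that character, enables the door's input and shows a text prompt, and leaving reverses the input and prompt.
; Pressing F inside the trigger checks the character's HasKey flag, then plays a timeline from the start that lerps the mesh's yaw to swing it open.
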(event `Key|F`
  (params (Key :type "Key Structure"))
  (:`Pressed`
    (if (`/Game/FirstPerson/Blueprints/BP_FirstPersonCharacter.Has key?` (stale `self.Box.OnComponentBeginOverlap` _asbp_first_person_character))
      (bind (_direction _doorfloat) (`Timeline|OpenDoorTimeline` :!via `PlayFromStart`)
        (:`Update`
          (`SceneComponent.K2_SetRelativeRotation` (`self.StaticMesh`) (`KismetMathLibrary.MakeRotator` 0.0 0.0 (`KismetMathLibrary.Lerp` 0.0 110.0 _doorfloat)) false false))))))

(event `self.Box.OnComponentBeginOverlap`
  (params (OverlappedComponent :type "PrimitiveComponent Object Reference") (OtherActor :type "Actor Object Reference") (OtherComp :type "PrimitiveComponent Object Reference") (OtherBodyIndex :type Integer) (bFromSweep :type Boolean) (SweepResult :type "HitResult Structure (by ref)"))
  (bind _asbp_first_person_character (cast `/Game/FirstPerson/Blueprints/BP_FirstPersonCharacter` OtherActor))
  (`self.EnableInput` (`GameplayStatics.GetPlayerController` 0))
  (`SceneComponent.SetVisibility` (`self.TextRender`) true false))

(event `self.Box.OnComponentEndOverlap`
  (params (OverlappedComponent :type "PrimitiveComponent Object Reference") (OtherActor :type "Actor Object Reference") (OtherComp :type "PrimitiveComponent Object Reference") (OtherBodyIndex :type Integer))
  (cast `/Game/FirstPerson/Blueprints/BP_FirstPersonCharacter` OtherActor)
  (`self.DisableInput` (`GameplayStatics.GetPlayerController` 0))
  (`SceneComponent.SetVisibility` (`self.TextRender`) false false))

(fn `UserConstructionScript`)